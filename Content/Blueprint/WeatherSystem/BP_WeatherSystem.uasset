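; Weather system actor, so far only a scaffold with no working weather or day/night behavior.
; The construction script moves the actor to the current world origin location, then runs nested validity checks on Sun, SkyLight, SkyAtmosphere and Fog that lead to no action.
; The event graph is empty, a rotation reset is disconnected, and DayLengthCurve and CurrentTime are unused.
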(fn `UserConstructionScript`
  (`self.K2_SetActorLocation` (`KismetMathLibrary.Conv_IntVectorToVector` (`GameplayStatics.GetWorldOriginLocation`)))
  (`/Engine/EditorBlueprintResources/StandardMacros.IsValid` (`self.Sun`)
    (:`Is Valid`
      (`/Engine/EditorBlueprintResources/StandardMacros.IsValid` (`self.SkyLight`)
        (:`Is Valid`
          (`/Engine/EditorBlueprintResources/StandardMacros.IsValid` (`self.SkyAtmosphere`)
            (:`Is Valid`
              (`/Engine/EditorBlueprintResources/StandardMacros.IsValid` (`self.Fog`)))))))))